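; BP_SequenceTrigger is a trigger volume that starts a level sequence when the first-person player character enters its box.
; The box overlap checks for BP_FirstPersonCharacter, then, if enabled, calls CallStartSequence with the assigned LevelSequence and itself as invoker.
; An optional one-time mode sets a Played flag on the first overlap, even when the trigger is disabled, so later overlaps do nothing.
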(event OnComponentBeginOverlap(Box)
  (params (OverlappedComponent :type Primitive%20Component%20Object%20Reference) (OtherActor :type Actor%20Object%20Reference) (OtherComp :type Primitive%20Component%20Object%20Reference) (OtherBodyIndex :type Integer) (bFromSweep :type Boolean) (SweepResult :type Hit%20Result%20Structure%20%28by%20ref%29))
  (Utilities|Casting|CastToBP_FirstPersonCharacter OtherActor)
  (if (Variables|Default|GetOneTimeOnly)
    (if (not (Variables|Default|GetPlayed))
      (Variables|Default|SetPlayed true)
      (if (Variables|Default|GetEnabled) :!label _label
        (Default|CallStartSequence (Variables|Default|GetLevelSequence) self)))
    (else
      (goto _label))))

(fn ConstructionScript)