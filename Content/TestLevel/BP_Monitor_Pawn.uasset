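; Interactable in-world monitor pawn that the player possesses to use a PC screen widget (WP_PCScreenD0).
; Interacting shows the cursor and disables interaction on the first-person character, with key presses forwarded through a WidgetInteraction component.
; The widget's exit button restores the original pawn and cancels the timer.
; If used during the first two minutes of game time, a one-minute timer plays the LS_J8Brzo sequence unless the player exits first.
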(event Custom|OnPressed_Event
  (bind _returnvalue (Game|GetPlayerController 0))
  (Variables|/Script/Engine.PlayerController|SetbShowMouseCursor _returnvalue false)
  (Pawn|Possess _returnvalue (Variables|Default|GetOriginalPawn))
  (bind _asbp_first_person_character (Utilities|Casting|CastToBP_FirstPersonCharacter (Variables|Default|GetOriginalPawn)))
  (Variables|/Game/FirstPerson/Blueprints/BP_FirstPersonCharacter.BP_FirstPersonCharacter_C|SetInteractiveEnabled _asbp_first_person_character true)
  (if (Class|KismetSystemLibrary|TimerExistsHandle (Variables|Default|GetTimer))
    (Utilities|Time|ClearandInvalidateTimerbyHandle (Variables|Default|GetTimer))))

(event Custom|Brzo
  (bind _outactor (Sequencer|Player|CreateLevelSequencePlayer "/Game/Audio/DAY0/J8Brzo/LS_J8Brzo.LS_J8Brzo"))
  (Sequencer|Player|Play (Variables|/Script/LevelSequence.LevelSequenceActor|GetSequencePlayer _outactor) :!class /Script/MovieScene.MovieSceneSequencePlayer))

(event EventOnInteract
  (params (invoker :type Actor%20Object%20Reference))
  (bind _returnvalue (Game|GetPlayerController 0))
  (Variables|/Script/Engine.PlayerController|SetbShowMouseCursor _returnvalue true)
  (Variables|Default|SetOriginalPawn (Pawn|GetControlledPawn _returnvalue))
  (Pawn|Possess _returnvalue self)
  (bind _asbp_first_person_character (Utilities|Casting|CastToBP_FirstPersonCharacter (Variables|Default|GetOriginalPawn)))
  (Variables|/Game/FirstPerson/Blueprints/BP_FirstPersonCharacter.BP_FirstPersonCharacter_C|SetInteractiveEnabled _asbp_first_person_character false)
  (if (< (Utilities|Time|GetGameTimeinSeconds) 1.2e+02)
    (if (Class|KismetSystemLibrary|TimerExistsHandle (Variables|Default|GetTimer))
      (Utilities|Time|ClearandInvalidateTimerbyHandle (Variables|Default|GetTimer)))
    (bind _returnvalue_2 (Utilities|Time|SetTimerbyEvent (delegate Custom|Brzo) 6e+01))
    (Variables|Default|SetTimer _returnvalue_2)))

(event EventBeginPlay
  (bind _aswp_pcscreen_d0 (Utilities|Casting|CastToWP_PCScreenD0 (UserInterface|GetWidget (Variables|Default|GetWidget))))
  (EventDispatchers|AssignOnPressed (Variables|/Game/UI/STAG/WP_PCScreenD0.WP_PCScreenD0_C|GetExitButton _aswp_pcscreen_d0) (delegate Custom|OnPressed_Event))
  (Default|CallInitEnded))

(event Input|KeyboardEvents|AnyKey
  (params (Key :type Key%20Structure :default "None"))
  (bind _widgetinteraction (Variables|Default|GetWidgetInteraction))
  (:Pressed
    (Class|WidgetInteractionComponent|PressPointerKey _widgetinteraction Key))
  (:Released
    (Class|WidgetInteractionComponent|ReleasePointerKey _widgetinteraction Key)))

(fn ConstructionScript)