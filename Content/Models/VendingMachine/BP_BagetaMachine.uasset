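; Interactable baguette vending machine that sells a baguette to the first-person character for one unit of money.
; BeginPlay sets a Czech interaction prompt, and OnInteract casts the invoker to BP_FirstPersonCharacter and checks its money.
; With money, it deducts one, spawns BP_Baguette at a fixed offset from the machine and calls BaguetteBought with the new actor.
; Without money, it calls BoughtWithouMoney instead.
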(event EventOnInteract
  (params (invoker :type Actor%20Object%20Reference))
  (bind _asbp_first_person_character (Utilities|Casting|CastToBP_FirstPersonCharacter invoker))
  (if (<= (Variables|/Game/FirstPerson/Blueprints/BP_FirstPersonCharacter.BP_FirstPersonCharacter_C|GetMoney _asbp_first_person_character) 0)
    (Default|CallBoughtWithouMoney)
    (else
      (bind _result (Math|Integer|DecrementInt (Variables|/Game/FirstPerson/Blueprints/BP_FirstPersonCharacter.BP_FirstPersonCharacter_C|GetMoney _asbp_first_person_character))
        (:%20%20
          (Default|SetMoneyCount _asbp_first_person_character _result)
          (bind _returnvalue (Game|SpawnActorfromClass "/Game/Models/Baguette/BP_Baguette.BP_Baguette_C" (Math|Transform|MakeTransform (+ (.location (Transformation|GetActorTransform self)) "-60.000000,60.000000,60.000000") "0, 0, 0" "1.000000,1.000000,1.000000") "Undefined" "MultiplyWithRoot" 0 0))
          (Default|CallBaguetteBought _returnvalue))))))

(event EventBeginPlay
  (Variables|Default|SetInteractText "Koupit bagetu"))

(fn ConstructionScript
  (|CallParentFunction))