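; BP_SubtitleManager is an actor that creates the WBP_Subtitles widget on BeginPlay and drives its on-screen subtitle text.
; It can show arbitrary text, clear the display, or step through a narration DataTable one row per ShowNextLine call.
; A FirstLine flag restarts at the first row of a given table, and the display clears once every row has been shown.
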(event Custom|ClearSubtitles
  (Default|DisplayLine (Variables|Default|GetSubitileWidget)))

(event Custom|ShowSubtitle
  (params (TextToShow :type Text))
  (Default|DisplayLine (Variables|Default|GetSubitileWidget) TextToShow))

(event Custom|ShowNextLine
  (params (FirstLine :type Boolean) (NarrationList :type Data%20Table%20Object%20Reference))
  (if FirstLine
    (Variables|Default|SetCurrent%20Narration%20List NarrationList)
    (Variables|Default|SetCurrentRow 0))
  (bind _outrownames (DataTable|GetDataTableRowNames (Variables|Default|GetCurrent%20Narration%20List)))
  (Variables|Default|SetRows _outrownames)
  (if (== (Variables|Default|GetCurrentRow) (Utilities|Array|Length (Variables|Default|GetRows)))
    (CallFunction|ClearSubtitles)
    (else
      (bind _returnvalue (Utilities|GetDataTableRow (Variables|Default|GetCurrent%20Narration%20List) (Utilities|Array|Get(acopy) (Variables|Default|GetRows) (Variables|Default|GetCurrentRow)))
        (:then
          (Default|DisplayLine (Variables|Default|GetSubitileWidget) (.LineToShow (Utilities|Struct|BreakStruct_Narration _returnvalue)))
          (Math|Integer|IncrementInt (Variables|Default|GetCurrentRow)))))))

(event EventBeginPlay
  (bind _returnvalue (UserInterface|CreateWidget "/Game/UI/WBP_Subtitles.WBP_Subtitles_C"))
  (bind _output_get (Variables|Default|SetSubitileWidget _returnvalue))
  (UserInterface|Viewport|AddtoViewport _output_get 0)
  (CallFunction|ClearSubtitles))

(fn ConstructionScript)